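; BP_Bullet is a projectile actor that travels in a straight line along its Direction at its Speed.
; Tick moves it by a frame-time-scaled offset without sweeping, so the move does no collision checks along the path.
; A short delay after BeginPlay arms the CanDamage flag, though no damage logic reads it here.
; The Puff! event prints a debug string and destroys the bullet.
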(event Custom|Puff!
  (Development|PrintString "PUFF!")
  (Actor|DestroyActor))

(event EventTick
  (params (DeltaSeconds :type Float%20%28single-precision%29))
  (Transformation|SetActorLocation (+ (Transformation|GetActorLocation) (* (* DeltaSeconds (Variables|Default|GetSpeed)) (Variables|Default|GetDirection))) false false))

(event EventBeginPlay
  (Utilities|FlowControl|Delay 0.2)
  (Variables|Default|SetCanDamage true))

(fn ConstructionScript)