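; BP_Firearm is a ranged weapon Blueprint that fires BP_BubbleRound projectiles from a muzzle point.
; Attacks decrement ammo, spawn a round at MuzzleLocation, then block further attacks for a cooldown, re-enabling only while ammo remains.
; Reloading waits the same cooldown before refilling ammo to full, with reload animation still a placeholder.
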(event EventBeginPlay
  (Variables|Default|SetAvailableAmmo (Variables|Default|GetAmmoSize)))

(event EventAttackImpl
  (Utilities|ReduceAmmo)
  (Game|SpawnActorfromClass "/Game/Blueprints/Weapons/BP_BubbleRound.BP_BubbleRound_C" (Transformation|GetWorldTransform (Variables|Default|GetMuzzleLocation)) "AlwaysSpawn" "MultiplyWithRoot" 0 0)
  (Variables|Default|SetCanAttack false)
  ;[0.15 0.15 0.15 0.5] Add Reload animation as well
  (Utilities|FlowControl|Delay (Variables|Default|GetCooldownTime))
  (Variables|Default|SetCanAttack (> (Variables|Default|GetAvailableAmmo) 0)))

(event EventReloadImpl
  ;[0.15 0.15 0.15 0.5] Placeholder for reload anim
  (Utilities|FlowControl|Delay (Variables|Default|GetCooldownTime))
  (Variables|Default|SetAvailableAmmo (Variables|Default|GetAmmoSize))
  (Variables|Default|SetCanAttack true))

(fn ConstructionScript
  (|CallParentFunction))