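; BP_Axe is a melee weapon Blueprint that deals area damage to pawns tagged Player.
; Its AttackImpl event runs a sphere overlap at the supplied location, using SphereTraceRadius, and applies Damage to each matching actor.
; It then clears CanAttack and restores it after a CooldownTime delay, whenever the overlap call has returned true.
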(event EventBeginPlay
  (|CallParentFunction) ; This node is disabled and will not be called.\nDrag off pins to build functionality.
)

(event EventAttackImpl
  (params (Direction :type Vector%20%28by%20ref%29 :default "0, 0, 0") (Location :type Vector :default "0, 0, 0") (Damage :type Float%20%28double-precision%29))
  ;[0.15 0.15 0.15 0.5] Sphere trace to get the enemy ahead
  (bind (_outactors _returnvalue) (Collision|SphereOverlapActors Location (Variables|Default|GetSphere%20Trace%20Radius) (Utilities|Array|MakeArray "ObjectTypeQuery3") 0))
  (if _returnvalue
    (for _array_element _outactors
      (if (Actor|ActorHasTag _array_element "Player")
        (Game|Damage|ApplyDamage _array_element (Variables|Default|GetDamage) 0 0))))
  (Variables|Default|SetCanAttack false)
  (Utilities|FlowControl|Delay (Variables|Default|GetCooldownTime))
  (Variables|Default|SetCanAttack true))

(fn ConstructionScript
  (|CallParentFunction))