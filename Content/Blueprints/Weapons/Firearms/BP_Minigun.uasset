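; Minigun firearm Blueprint that adds spin-up timing and audio to the inherited attack.
; An attack at full ammo activates the audio, waits for the wind-up delay and triggers the fire-start sound before calling the parent attack.
; Attacks below full ammo go straight to the parent, and running out of ammo triggers the stop sound.
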(event EventOnOutOfAmmo
  (Class|AudioParameterControllerInterface|SetTriggerParameter (Variables|Default|GetAudio) "Minigun_Stop"))

(event EventAttackImpl
  (params (Direction :type Vector%20%28by%20ref%29 :default "0, 0, 0") (Location :type Vector :default "0, 0, 0") (Damage :type Float%20%28double-precision%29))
  (if (== (Variables|Default|GetAvailableAmmo) (Variables|Default|GetAmmoSize))
    (Components|Activation|Activate (Variables|Default|GetAudio) false)
    (Utilities|FlowControl|Delay (Variables|Default|GetWindUp))
    (Class|AudioParameterControllerInterface|SetTriggerParameter (Variables|Default|GetAudio) "MG_FireStart"))
  (|CallParentFunction Direction Location Damage))

(fn ConstructionScript
  (|CallParentFunction))