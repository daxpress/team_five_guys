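; Shotgun firearm Blueprint that spawns a bullet at its muzzle when attacking.
; AttackImpl passes direction and damage to the bullet, then blocks further attacks.
; A timeline kicks the owning BP_Duck's WeaponChild pitch for recoil.
; When it finishes, a cooldown re-enables attacking if ammo remains, otherwise it triggers the out-of-ammo handler.
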(event EventBeginPlay
  (|CallParentFunction) ; This node is disabled and will not be called.\nDrag off pins to build functionality.
)

(event Collision|EventActorBeginOverlap
  (params (OtherActor :type Actor%20Object%20Reference)))

(event EventAttackImpl
  (params (Direction :type Vector%20%28by%20ref%29 :default "0, 0, 0") (Location :type Vector :default "0, 0, 0") (Damage :type Float%20%28double-precision%29))
  (Game|SpawnActorfromClass (Variables|Default|GetBulletClass) (Transformation|GetWorldTransform (Variables|Default|GetMuzzleLocation)) "AlwaysSpawn" "MultiplyWithRoot" (Actor|GetParentActor) Damage Direction 0)
  (Variables|Default|SetCanPerformAttack false)
  (Variables|Default|SetShooting true)
  (bind _newtrack_0 (Timeline|Timeline PlayFromStart)
    (:Update
      (Transformation|SetRelativeRotation (Variables|/Game/Blueprints/Characters/BP_Duck.BP_Duck_C|GetWeaponChild (.AsBP%20Duck (Utilities|Casting|CastToBP_Duck (Actor|GetParentActor)))) (Math|Rotator|MakeRotator 0.0 (* _newtrack_0 5e+01) 0.0) false false))
    (:Finished
      (Utilities|FlowControl|Delay (Variables|Default|GetCooldownTime))
      (Variables|Default|SetShooting false)
      (bind _output_get (Variables|Default|SetCanPerformAttack (> (Variables|Default|GetAvailableAmmo) 0)))
      (if (not _output_get)
        (CallFunction|OnOutOfAmmo)))))

(fn ConstructionScript
  (|CallParentFunction))