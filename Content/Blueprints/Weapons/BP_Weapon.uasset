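; BP_Weapon is a weapon Blueprint that fires BP_BubbleRound projectiles from its MuzzleLocation and tracks limited ammo.
; Attack checks CanShoot, decrements ammo, spawns a round, then re-enables firing after a cooldown only if ammo remains.
; Reload waits the same cooldown time, then refills ammo and re-enables shooting, with its animation still a placeholder.
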(event EventAttack
  (if (Variables|Default|GetCanShoot)
    (Utilities|ReduceAmmo)
    (Game|SpawnActorfromClass "/Game/Blueprints/Weapons/BP_BubbleRound.BP_BubbleRound_C" (Transformation|GetWorldTransform (Variables|Default|GetMuzzleLocation)) "AlwaysSpawn" "MultiplyWithRoot" 0 0)
    (Variables|Default|SetCanShoot false)
    ;[0.15 0.15 0.15 0.5] Add Reload animation as well
    (Utilities|FlowControl|Delay (Variables|Default|GetCooldownTime))
    (Variables|Default|SetCanShoot (> (Variables|Default|GetAvailableAmmo) 0))))

(event EventReload
  ;[0.15 0.15 0.15 0.5] Placeholder for reload anim
  (Utilities|FlowControl|Delay (Variables|Default|GetCooldownTime))
  (Variables|Default|SetAvailableAmmo (Variables|Default|GetAmmoSize))
  (Variables|Default|SetCanShoot true))

(event EventBeginPlay
  (Variables|Default|SetAvailableAmmo (Variables|Default|GetAmmoSize)))

(fn ConstructionScript)