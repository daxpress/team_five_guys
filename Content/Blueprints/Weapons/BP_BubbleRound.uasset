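; Bubble projectile actor for a weapon that flies straight and damages what it touches.
; Tick moves it along its forward vector at Speed without sweeping, so hits rely on the Sphere's begin-overlap event.
; A short arming delay after BeginPlay enables damage; an armed overlap applies Damage to the other actor, then calls Puff, which prints a message and destroys the bubble.
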(event OnComponentBeginOverlap(Sphere)
  (params (OverlappedComponent :type Primitive%20Component%20Object%20Reference) (OtherActor :type Actor%20Object%20Reference) (OtherComp :type Primitive%20Component%20Object%20Reference) (OtherBodyIndex :type Integer) (bFromSweep :type Boolean) (SweepResult :type Hit%20Result%20Structure%20%28by%20ref%29))
  (if (Variables|Default|GetCanDamage)
    (Game|Damage|ApplyDamage OtherActor (Variables|Default|GetDamage) 0 0)
    (CallFunction|Puff!)))

(event Custom|Puff!
  (Development|PrintString "PUFF!")
  (Actor|DestroyActor))

(event EventTick
  (params (DeltaSeconds :type Float%20%28single-precision%29))
  (Transformation|SetActorLocation (+ (Transformation|GetActorLocation) (* (* DeltaSeconds (Variables|Default|GetSpeed)) (Transformation|GetActorForwardVector))) false false))

(event EventBeginPlay
  (Utilities|FlowControl|Delay 0.2)
  (Variables|Default|SetCanDamage true))

(fn ConstructionScript)