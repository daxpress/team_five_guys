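; BP_Duck is a damageable duck character that carries a weapon in a child actor and dies when its health runs out.
; On BeginPlay it stores the child actor as a BPI_Attack weapon reference, and only if that cast succeeds sets Health to MaxHealth.
; Incoming damage reduces Health, and at zero it prints a quack, spawns a Niagara explosion at its transform and destroys itself.
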(event Custom|ManageHealth
  (params (Damage :type Float%20%28double-precision%29))
  (bind _output_get (Variables|Health|SetHealth (- (Variables|Health|GetHealth) Damage)))
  (if (<= _output_get 0.0)
    (CallFunction|Death)))

(event Custom|Death
  (bind _returnvalue (Transformation|GetActorTransform))
  (Development|PrintString "QUAAACK!!")
  (Niagara|SpawnSystematLocation "/Game/sA_StylizedMix/Fx/NS_Smokeless_StylizedExplosion_1.NS_Smokeless_StylizedExplosion_1" (.location _returnvalue) (.rotation _returnvalue) (.scale _returnvalue) true true "AutoRelease")
  (Actor|DestroyActor))

(event EventBeginPlay
  (bind _asbpi_attack (Utilities|Casting|CastToBPI_Attack (Variables|/Script/Engine.ChildActorComponent|GetChildActor (Variables|Default|GetChildActor))))
  (Variables|Weapon|SetWeaponReference _asbpi_attack)
  (Variables|Health|SetHealth (Variables|Health|GetMaxHealth)))

(event Game|Damage|EventAnyDamage
  (params (Damage :type Float%20%28single-precision%29) (DamageType :type Damage%20Type%20Object%20Reference) (InstigatedBy :type Controller%20Object%20Reference) (DamageCauser :type Actor%20Object%20Reference))
  (CallFunction|ManageHealth Damage))

(fn ConstructionScript)