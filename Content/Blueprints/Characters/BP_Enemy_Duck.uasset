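; BP_Enemy_Duck is a duck enemy character that attacks the player with a weapon and shows its health on a widget bar.
; AttackPlayer aims from the weapon's attack origin toward the player's location, passing that direction and the melee attack point's world location to the weapon.
; ManageHealth runs the parent logic, then updates the HP bar's fill from current over maximum health.
; ReloadWeapon forwards to the referenced weapon.
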(event Custom|ReloadWeapon
  (Default|Reload (Variables|Default|GetWeaponReference)))

(event EventBeginPlay
  (|CallParentFunction) ; This node is disabled and will not be called.\nDrag off pins to build functionality.
)

(event EventManageHealth
  (params (Damage :type Float%20%28double-precision%29))
  (|CallParentFunction Damage)
  (bind _aswb_enemy_hpbar (Utilities|Casting|CastToWB_EnemyHPBar (UserInterface|GetWidget (Variables|Default|GetHPBarWidget))))
  (Progress|SetPercent (Variables|/Game/Blueprints/Widgets/WB_EnemyHPBar.WB_EnemyHPBar_C|GetEnemyHP _aswb_enemy_hpbar) (/ (Variables|Default|GetHealth) (Variables|Default|GetMaxHealth))))

(fn ConstructionScript
  (|CallParentFunction))

(fn AttackPlayer
  (params (PlayerLocation :type Vector) (Weapon :type BPI%20Attack%20Interface))
  (bind _location (Default|GetAttackOrigin Weapon))
  (bind _success (Default|Attack Weapon (Math|Vector|Normalize (- PlayerLocation _location)) (Transformation|GetWorldLocation (Variables|Default|GetMeleeAttackLocation))))
  (return _success))