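; AI controller for the duck enemy that runs its behavior tree and feeds it the player as a target.
; On possessing a duck enemy pawn, it stores the pawn, starts BT_Duck and zeroes the Range blackboard key.
; AI Perception updates set the Target key when a Player-tagged actor is successfully sensed; this controller never clears that key when sensing is lost.
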(event OnTargetPerceptionUpdated(AIPerception)
  (params (Actor :type Actor%20Object%20Reference) (Stimulus :type AI%20Stimulus%20Structure))
  (if (and (Actor|ActorHasTag Actor "Player") (.bsuccessfullysensed Stimulus))
    (AI|Components|Blackboard|SetValueasObject (Variables|Default|GetBlackboard) (Utilities|Name|MakeLiteralName "Target") Actor)))

(event EventPossess
  (params (PossessedPawn :type Pawn%20Object%20Reference))
  (bind _asbp_enemy_duck (Utilities|Casting|CastToBP_Enemy_Duck PossessedPawn))
  (Variables|Default|SetControlled _asbp_enemy_duck)
  (AI|RunBehaviorTree "/Game/Blueprints/Characters/BehaviourTrees/BT_Duck.BT_Duck")
  (AI|Components|Blackboard|SetValueasFloat (Variables|Default|GetBlackboard) (Utilities|Name|MakeLiteralName "Range") 0.0))

(fn ConstructionScript)