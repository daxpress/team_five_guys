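; Modular interior wall piece for building houses, configured entirely in the Construction Script with no active runtime logic.
; The WallIn enum indexes straight and bent mesh arrays in A or B styles to set the wall mesh.
; Optional flags add a doorframe child actor on door variants and corner decal meshes on doors, columns and outer corners, destroying the decal otherwise.
; RevertDefaultMaterials acts as a self-resetting toggle that restores the mesh's default materials.
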(event EventBeginPlay)

(event Collision|EventActorBeginOverlap
  (params (OtherActor :type Actor%20Object%20Reference)))

(event EventTick
  (params (DeltaSeconds :type Float%20%28single-precision%29)))

(fn ConstructionScript
  (bind _returnvalue (Math|Transform|MakeTransform "0,-150.000000,0.000000"))
  (bind _wallin (Variables|Mesh|GetWallIn))
  (bind _bent_interior_wall (Variables|Mesh|GetBent%20Interior%20Wall))
  (bind _wallin_mesh (Variables|Default|GetWallIn_mesh))
  ;[1 1 1] WallIn Mesh Assign
  (if (Variables|Mesh|GetWallIn_B)
    (if _bent_interior_wall
      (Components|StaticMesh|SetStaticMesh (Variables|Default|GetWallIn_mesh) (Utilities|Array|Get(acopy) (Variables|Mesh|GetWall%20in%20B%20Bent%20Meshes) (Math|Conversions|ToInteger(Byte) (Variables|Mesh|GetWallIn))))
      (else
        (Components|StaticMesh|SetStaticMesh (Variables|Default|GetWallIn_mesh) (Utilities|Array|Get(acopy) (Variables|Mesh|GetWall%20in%20B%20Meshes) (Math|Conversions|ToInteger(Byte) (Variables|Mesh|GetWallIn))))))
    (elif _bent_interior_wall
      (Components|StaticMesh|SetStaticMesh (Variables|Default|GetWallIn_mesh) (Utilities|Array|Get(acopy) (Variables|Mesh|GetWall%20in%20A%20Bent%20Meshes) (Math|Conversions|ToInteger(Byte) (Variables|Mesh|GetWallIn))))
      (else
        (Components|StaticMesh|SetStaticMesh (Variables|Default|GetWallIn_mesh) (Utilities|Array|Get(acopy) (Variables|Mesh|GetWall%20in%20A%20Meshes) (Math|Conversions|ToInteger(Byte) (Variables|Mesh|GetWallIn)))))))
  ;[1 1 1] Doorframe
  (if (Variables|Mesh|GetDoorframe)
    (switch Utilities|FlowControl|Switch|SwitchonE_WallIn (Variables|Mesh|GetWallIn)
      (:NewEnumerator19
        _)
      (:NewEnumerator25
        _)
      (:NewEnumerator26
        _)
      (:NewEnumerator27
        (AddComponent|AddChildActorComponent false _returnvalue))
      (:NewEnumerator28
        (AddComponent|AddChildActorComponent false _returnvalue))
      (:NewEnumerator29
        _)
      (:NewEnumerator30
        _)
      (:NewEnumerator31
        _)
      (:NewEnumerator32
        _)
      (:NewEnumerator33
        _)
      (:NewEnumerator34
        _)
      (:NewEnumerator35
        _)
      (:NewEnumerator36
        _)
      (:NewEnumerator37
        _)
      (:NewEnumerator38
        _)
      (:NewEnumerator39
        _)
      (:NewEnumerator40
        _)
      (:NewEnumerator41
        _)
      (:NewEnumerator42
        _)
      (:NewEnumerator43
        _)))
  ;[1 1 1] Corner Decals
  (if (Variables|Mesh|GetDecal_corner)
    (if (Variables|Mesh|GetWallIn_B)
      (switch Utilities|FlowControl|Switch|SwitchonE_WallIn _wallin
        (:NewEnumerator19
          (Components|DestroyComponent (Variables|Default|GetDecal_corner_mesh) :!label _label))
        (:NewEnumerator25
          (goto _label))
        (:NewEnumerator26
          (goto _label))
        (:NewEnumerator27
          (Components|StaticMesh|SetStaticMesh (Variables|Default|GetDecal_corner_mesh) (Utilities|Array|Get(acopy) (Variables|Mesh|GetDecal%20Corner%20B%20Meshes) (Math|Conversions|ToInteger(Byte) (Variables|Mesh|GetWallIn))) :!label _label_2))
        (:NewEnumerator28
          (goto _label_2))
        (:NewEnumerator29
          (goto _label))
        (:NewEnumerator30
          (goto _label))
        (:NewEnumerator31
          (goto _label))
        (:NewEnumerator32
          (goto _label))
        (:NewEnumerator33
          (goto _label))
        (:NewEnumerator34
          (goto _label))
        (:NewEnumerator35
          (goto _label_2))
        (:NewEnumerator36
          (goto _label_2))
        (:NewEnumerator37
          (goto _label_2))
        (:NewEnumerator38
          (goto _label_2))
        (:NewEnumerator39
          (goto _label_2))
        (:NewEnumerator40
          (goto _label_2))
        (:NewEnumerator41
          (goto _label_2))
        (:NewEnumerator42
          (goto _label_2))
        (:NewEnumerator43
          (goto _label_2)))
      (else
        (switch Utilities|FlowControl|Switch|SwitchonE_WallIn _wallin
          (:NewEnumerator19
            (goto _label))
          (:NewEnumerator25
            (goto _label))
          (:NewEnumerator26
            (goto _label))
          (:NewEnumerator27
            _)
          (:NewEnumerator28
            _)
          (:NewEnumerator29
            (goto _label))
          (:NewEnumerator30
            (goto _label))
          (:NewEnumerator31
            (goto _label))
          (:NewEnumerator32
            (goto _label))
          (:NewEnumerator33
            (goto _label))
          (:NewEnumerator34
            (goto _label))
          (:NewEnumerator35
            _)
          (:NewEnumerator36
            _)
          (:NewEnumerator37
            _)
          (:NewEnumerator38
            _)
          (:NewEnumerator39
            _)
          (:NewEnumerator40
            _)
          (:NewEnumerator41
            _)
          (:NewEnumerator42
            _)
          (:NewEnumerator43
            _))
        (Components|StaticMesh|SetStaticMesh (Variables|Default|GetDecal_corner_mesh) (Utilities|Array|Get(acopy) (Variables|Mesh|GetDecal%20Corner%20A%20Meshes) (Math|Conversions|ToInteger(Byte) (Variables|Mesh|GetWallIn))))))
    (else
      (goto _label)))
  ;[1 1 1] Revert Materials
  (if (Variables|Mesh|GetRevert%20Default%20Materials)
    (bind _output_get (LocalVariables|SetNumber%20Of%20Materials (Rendering|Material|GetNumMaterials _wallin_mesh)))
    (for _index (range 0 _output_get)
      (Rendering|Material|SetMaterial _wallin_mesh _index (Rendering|Material|GetMaterial (Variables|/Script/Engine.StaticMeshComponent|GetStaticMesh _wallin_mesh) _index)))
    (Variables|Mesh|SetRevert%20Default%20Materials false)))