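; BP_SpawnCurvedShield is a VFX spawner that repeatedly creates BP_Curved_Shield actors at its own location and rotation.
; BeginPlay starts a spawn loop, and the custom Again event repeats it every eight seconds with no exit condition.
; Each spawn receives the spawner's variables for shield actor, material, random rotation, particle amount and size, colors, and scale.
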(event Custom|Again
  (Game|SpawnActorfromClass "/Game/Stylized_VFX_StPack/Blueprints/BP_Curved_Shield.BP_Curved_Shield_C" (Math|Transform|MakeTransform (Transformation|GetActorLocation) (Transformation|GetActorRotation) "1,1,1") "Undefined" 0 (Variables|Default|GetActor_Shield) (Variables|Default|GetMI_Shield_Material) (Variables|Default|GetRandomRotation) (Variables|Default|GetParticles_Amount) (Variables|Default|GetParticles_Size) (Variables|Default|GetOutsideColor) (Variables|Default|GetInsideColor) "(R=0.786458,G=0.571834,B=0.038624,A=1.000000)" 6.0 (Variables|Default|GetScale) true 2 0)
  (Utilities|FlowControl|Delay 8.0)
  (CallFunction|Again))

(event EventBeginPlay
  (Game|SpawnActorfromClass "/Game/Stylized_VFX_StPack/Blueprints/BP_Curved_Shield.BP_Curved_Shield_C" (Math|Transform|MakeTransform (Transformation|GetActorLocation) (Transformation|GetActorRotation) "1,1,1") "Undefined" 0 (Variables|Default|GetActor_Shield) (Variables|Default|GetMI_Shield_Material) (Variables|Default|GetRandomRotation) (Variables|Default|GetParticles_Amount) (Variables|Default|GetParticles_Size) (Variables|Default|GetOutsideColor) (Variables|Default|GetInsideColor) "(R=0.786458,G=0.571834,B=0.038624,A=1.000000)" 6.0 (Variables|Default|GetScale) true 2 0)
  (Utilities|FlowControl|Delay 8.0)
  (CallFunction|Again))

(fn ConstructionScript)