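; Spawner actor for the stylized VFX pack that places a BP_Portal effect at its own transform when play begins.
; It passes its Endless and Duration settings to the spawned portal.
; When not endless, it waits for the portal's duration plus a short buffer, then calls its Again event to spawn a new one, looping the effect indefinitely.
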(event Custom|Again
  (Game|SpawnActorfromClass "/Game/Stylized_VFX_StPack/Blueprints/UPDATE_1_2/BP_Portal.BP_Portal_C" (Transformation|GetActorTransform) "Undefined" 0 (Variables|Default|GetbEndless?) (Variables|Default|GetDuration) 0)
  (if (not (Variables|Default|GetbEndless?))
    (Utilities|FlowControl|Delay (+ (Variables|Default|GetDuration) 3.0))
    (CallFunction|Again)))

(event EventBeginPlay
  (Game|SpawnActorfromClass "/Game/Stylized_VFX_StPack/Blueprints/UPDATE_1_2/BP_Portal.BP_Portal_C" (Transformation|GetActorTransform) "Undefined" 0 (Variables|Default|GetbEndless?) (Variables|Default|GetDuration) 0)
  (if (not (Variables|Default|GetbEndless?))
    (Utilities|FlowControl|Delay (+ (Variables|Default|GetDuration) 3.0))
    (CallFunction|Again)))

(fn ConstructionScript)