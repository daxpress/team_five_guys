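; Spawner actor from a stylized VFX pack that repeatedly launches web projectiles at its own transform.
; On BeginPlay it waits a delay scaled by its Level, then spawns a BP_Web_Projectile, passing along its Gravity, ImpulsePower and Level values.
; A self-calling Again event then repeats the spawn on a fixed delay for an endless loop.
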(event Custom|Again
  (Utilities|FlowControl|Delay 6.0)
  (Game|SpawnActorfromClass "/Game/Stylized_VFX_StPack/Blueprints/UPDATE_1_3/BP_Web_Projectile.BP_Web_Projectile_C" (Transformation|GetActorTransform) "Undefined" 0 (Variables|Default|GetbGravity) (Variables|Default|GetImpulse%20Power) (Variables|Default|GetLevel) 0)
  (CallFunction|Again))

(event EventBeginPlay
  (Utilities|FlowControl|Delay (* (Variables|Default|GetLevel) 2.0))
  (Game|SpawnActorfromClass "/Game/Stylized_VFX_StPack/Blueprints/UPDATE_1_3/BP_Web_Projectile.BP_Web_Projectile_C" (Transformation|GetActorTransform) "Undefined" 0 (Variables|Default|GetbGravity) (Variables|Default|GetImpulse%20Power) (Variables|Default|GetLevel) 0)
  (CallFunction|Again))

(fn ConstructionScript)