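; BP_SpawnShieldv2 is a spawner actor in the Stylized VFX pack that repeatedly spawns one of three Shieldv2 effect Blueprints at its own transform.
; Its Level variable selects the shield variant and also scales the initial BeginPlay delay, staggering spawners of different levels.
; After each spawn, the Again event waits a fixed interval and calls itself, forming an endless respawn loop.
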(event Custom|Again
  (bind _returnvalue (Transformation|GetActorTransform))
  (switch int (Variables|Default|GetLevel)
    (:1
      (Game|SpawnActorfromClass "/Game/Stylized_VFX_StPack/Blueprints/UPDATE_1_3/BP_Shieldv2_01.BP_Shieldv2_01_C" _returnvalue "Undefined" 0 4.0 1.2 "(R=1.000000,G=0.806952,B=0.000000,A=1.000000)" "(R=0.807292,G=0.176150,B=0.000000,A=1.000000)" true 1 0))
    (:2
      (Game|SpawnActorfromClass "/Game/Stylized_VFX_StPack/Blueprints/UPDATE_1_3/BP_Shieldv2_02.BP_Shieldv2_02_C" _returnvalue "Undefined" 0 6.0 1.5 "(R=0.000000,G=1.000000,B=0.904661,A=1.000000)" "(R=0.807292,G=0.575449,B=0.000000,A=1.000000)" true 2 0))
    (:3
      (Game|SpawnActorfromClass "/Game/Stylized_VFX_StPack/Blueprints/UPDATE_1_3/BP_Shieldv2_03.BP_Shieldv2_03_C" _returnvalue "Undefined" 0 1e+01 1.7 "(R=0.371238,G=0.020289,B=1.000000,A=1.000000)" "(R=0.000000,G=0.240132,B=0.515625,A=1.000000)" true 3 0)))
  (Utilities|FlowControl|Delay 8.0)
  (CallFunction|Again))

(event EventBeginPlay
  (bind _returnvalue (Transformation|GetActorTransform))
  (Utilities|FlowControl|Delay (* (Variables|Default|GetLevel) 0.5))
  (switch int (Variables|Default|GetLevel)
    (:1
      (Game|SpawnActorfromClass "/Game/Stylized_VFX_StPack/Blueprints/UPDATE_1_3/BP_Shieldv2_01.BP_Shieldv2_01_C" _returnvalue "Undefined" 0 4.0 1.2 "(R=1.000000,G=0.806952,B=0.000000,A=1.000000)" "(R=0.807292,G=0.176150,B=0.000000,A=1.000000)" true 1 0))
    (:2
      (Game|SpawnActorfromClass "/Game/Stylized_VFX_StPack/Blueprints/UPDATE_1_3/BP_Shieldv2_02.BP_Shieldv2_02_C" _returnvalue "Undefined" 0 6.0 1.5 "(R=0.000000,G=1.000000,B=0.904661,A=1.000000)" "(R=0.807292,G=0.575449,B=0.000000,A=1.000000)" true 2 0))
    (:3
      (Game|SpawnActorfromClass "/Game/Stylized_VFX_StPack/Blueprints/UPDATE_1_3/BP_Shieldv2_03.BP_Shieldv2_03_C" _returnvalue "Undefined" 0 1e+01 1.7 "(R=0.371238,G=0.020289,B=1.000000,A=1.000000)" "(R=0.000000,G=0.240132,B=0.515625,A=1.000000)" true 3 0)))
  (Utilities|FlowControl|Delay 8.0)
  (CallFunction|Again))

(fn ConstructionScript)